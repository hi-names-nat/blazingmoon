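; BP_BMPlayerController is a player controller that owns the on-screen dialogue widget.
; BeginPlay creates one instance from the DialogueWidget class and keeps it in WidgetInstance.
; DrawDialogue and RemoveDialogue add that instance to the player screen or take it off.
; SetDialogueText casts it to WBP_DialogueScreen and passes the text on, doing nothing if the cast fails.
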(event EventBeginPlay
  (bind _returnvalue (UserInterface|CreateWidget (Variables|Default|GetDialogueWidget)))
  (Variables|Default|SetWidgetInstance _returnvalue))

(event EventTick
  (params (DeltaSeconds :type Float%20%28single-precision%29)))

(fn ConstructionScript)

(fn DrawDialogue
  (UserInterface|Viewport|AddtoPlayerScreen (Variables|Default|GetWidgetInstance)))

(fn RemoveDialogue
  (Widget|RemovefromParent (Variables|Default|GetWidgetInstance)))

(fn SetDialogueText
  (params (Text :type String))
  (bind _aswbp_dialogue_screen (Utilities|Casting|CastToWBP_DialogueScreen (Variables|Default|GetWidgetInstance)))
  (Default|SetText _aswbp_dialogue_screen Text))